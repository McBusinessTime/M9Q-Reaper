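; Enemy character for the MQ9Reaper game that takes damage, dies and awards score to the drone that killed it.
; While alive, incoming damage reduces Health; at zero or below, the mesh switches to physics simulation and IsAlive is cleared.
; If the damage causer is an MQ9Reaper_BP, ScoreGiven is added to its DroneUI Score and TotalScore, and the score pop-in animation plays.
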(event `self.ReceiveAnyDamage`
  (params (Damage :type "Float (single-precision)") (DamageType :type "DamageType Object Reference") (InstigatedBy :type "Controller Object Reference") (DamageCauser :type "Actor Object Reference"))
  (if (`self.IsAlive`)
    ;[1 1 1] Health/Death logic
    (bind _output_get (set `self.Health` (- (`self.Health`) Damage)))
    (`/Engine/EditorBlueprintResources/StandardMacros.CompareFloat` _output_get
      (:`==`
        _)
      (:`<`
        _))
    (`PrimitiveComponent.SetSimulatePhysics` (`self.Mesh`) true)
    (set `self.IsAlive` false)
    ;[1 1 1] Cast to MQ9Reaper
    (bind _asmq9reaper_bp (cast `/Game/MQ9Reaper/Blueprint/MQ9Reaper_BP` DamageCauser))
    (bind _droneui (`/Game/MQ9Reaper/Blueprint/MQ9Reaper_BP.DroneUI` _asmq9reaper_bp))
    ;[1 1 1] Add given score to DroneUI score/total score
    (set `/Game/MQ9Reaper/Blueprint/Widgets/DroneUI.Score` (+ (`/Game/MQ9Reaper/Blueprint/Widgets/DroneUI.Score` _droneui) (`self.ScoreGiven`)) _droneui)
    (set `/Game/MQ9Reaper/Blueprint/Widgets/DroneUI.TotalScore` (+ (`/Game/MQ9Reaper/Blueprint/Widgets/DroneUI.TotalScore` _droneui) (`self.ScoreGiven`)) _droneui)
    ;[1 1 1] Play score popin animation
    (`/Game/MQ9Reaper/Blueprint/Widgets/DroneUI.PlayScorePopin` _droneui)))

(fn `UserConstructionScript`)