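; Missile actor for the MQ9 Reaper that launches from a wing and explodes on hit or overlap.
; MissileFire aims velocity by wing rotation, turns on trail, light, sounds and material glow, and arms a start-closed DoOnce.
; The armed explosion applies radial damage and physics impulses scaled from damage settings, then delays destruction so particles finish.
; HomingLerp uses a timeline to ramp homing acceleration.
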(event `self.ReceiveHit`
  (params (MyComp :type "PrimitiveComponent Object Reference") (Other :type "Actor Object Reference") (OtherComp :type "PrimitiveComponent Object Reference") (bSelfMoved :type Boolean) (HitLocation :type "Vector Structure") (HitNormal :type "Vector Structure") (NormalImpulse :type "Vector Structure") (Hit :type "HitResult Structure (by ref)"))
  ;[0 0 0] Missile Explode events
  ;;[1 1 1] If hit or overlap actors/components that is not self
  (if (!= (stale `self.ReceiveActorBeginOverlap` OtherActor) (`self.SelfReference`)) :!label _label
    ;;[1 1 1] Unlock explode events
    (`/Engine/EditorBlueprintResources/StandardMacros.DoOnce` true :!label _label_2
      (:`Completed`
        ;;[1 1 1] Set Hit location
        (set `self.HitLocation` (`self.K2_GetActorLocation`))
        ;;[1 1 1] Spawn explosion at hit location
        (`GameplayStatics.SpawnEmitterAtLocation` (`self.ExplosionParticle`) (`self.HitLocation`))
        ;;[1 1 1] Deactivate missile trail
        (`ActorComponent.Deactivate` (`self.MissileTrail`))
        ;;[1 1 1] Apply radial damage at hit location
        (`GameplayStatics.ApplyRadialDamage` :`BaseDamage` (`self.Damage`) :`Origin` (`self.HitLocation`) :`DamageRadius` (`self.DamageRadius`) :`DamageCauser` (`self.SelfReference`))
        ;;[1 1 1] Destroy missile components and play explosion sound
        (`ActorComponent.K2_DestroyComponent` (`self.ProjectileMesh`))
        (`ActorComponent.K2_DestroyComponent` (`self.MissileLight`))
        (`ActorComponent.K2_DestroyComponent` (`self.Loop`))
        (`GameplayStatics.PlaySoundAtLocation` "/Game/MQ9Reaper/Audio/Wav/Explosion01.Explosion01" (`self.HitLocation`) (struct) 1.0 1.0 0.0 "/Game/MQ9Reaper/Audio/ExlosiveAttenuation.ExlosiveAttenuation")
        ;;[1 1 1] Get components within range around radius
        (bind _outcomponents (`KismetSystemLibrary.SphereOverlapComponents_NEW` (`self.HitLocation`) (* (`self.DamageRadius`) 1.5) (`|MakeArray` "ObjectTypeQuery1" "ObjectTypeQuery3" "ObjectTypeQuery4" "ObjectTypeQuery2" :!type "EObjectTypeQuery Enum")))
        ;;[1 1 1] Apply radial physics, dependant on Damage and Damage radius
        (for _array_element _outcomponents
          (`PrimitiveComponent.AddRadialImpulse` _array_element (`self.HitLocation`) (* (`self.DamageRadius`) 1.5) (* (`self.Damage`) 2.0) "RIF_Constant" true))
        ;;[1 1 1] Delay before destroying actor, to allow particle animations to finish
        (`KismetSystemLibrary.Delay` 5.0)
        (`self.K2_DestroyActor`)))))

(event `self.ReceiveActorBeginOverlap`
  (params (OtherActor :type "Actor Object Reference"))
  ;[0 0 0] Missile Explode events
  ;;[1 1 1] If hit or overlap actors/components that is not self
  (goto _label))

(event `MissileFire`
  ;[0 0 0] Missile Fire events
  ;;[1 1 1] Activates when you fire missile
  (`|ExecutionSequence`
    (:`then_0`
      (goto _label_2 :!via `Reset`))
    (:`then_1`
      ;;[1 1 1] Set projectile velocity direction from wing rotation
      (set `self.IsDetached` true)
      (set `MovementComponent.Velocity` (`KismetMathLibrary.GreaterGreater_VectorRotator` (`MovementComponent.Velocity` (`self.ProjectileMovement`)) (`SceneComponent.K2_GetComponentRotation` (`self.WingReference`))) (`self.ProjectileMovement`))
      ;;[1 1 1] Set emissive strength for missile material
      (`MaterialInstanceDynamic.SetScalarParameterValue` (`self.MissileMaterialInstance`) "RocketPower" 5000.0)
      ;;[1 1 1] Activate particle system and light
      (`ActorComponent.Activate` (`self.MissileTrail`) false)
      (`SceneComponent.SetVisibility` (`self.MissileLight`) true false)
      ;;[1 1 1] Play fire sound
      (`GameplayStatics.PlaySoundAtLocation` "/Game/MQ9Reaper/Audio/Wav/Missile_08.Missile_08" (`self.K2_GetActorLocation`) (struct) 1.0 (`KismetMathLibrary.RandomFloatInRange` 0.5 1.0) 0.0 "/Game/MQ9Reaper/Audio/FarRangeAttenuation.FarRangeAttenuation")
      ;;[1 1 1] Set random pitch for loop
      (`AudioComponent.SetPitchMultiplier` (`self.Loop`) (`KismetMathLibrary.RandomFloatInRange` 0.6 0.8))
      ;;[1 1 1] Set volume to audible for loop
      (`AudioComponent.SetVolumeMultiplier` (`self.Loop`) 1.0))))

(event `HomingLerp`
  ;[0 0 0] Homing Lerp Logic
  (bind (_direction _hominglerp) (`Timeline|HomingLerpTimeline`)
    (:`Update`
      (bind _output_get (set `self.HomingLerpFloat` _hominglerp))
      (set `ProjectileMovementComponent.HomingAccelerationMagnitude` (`KismetMathLibrary.Lerp` 0.0 50000.0 _output_get) (`self.ProjectileMovement`)))))

(fn `UserConstructionScript`
  (bind _projectilemesh (`self.ProjectileMesh`))
  ;[0 0 0] Create and set dynamic materials and set emissive power to 0
  (bind _returnvalue (`PrimitiveComponent.CreateDynamicMaterialInstance` _projectilemesh 0 (`PrimitiveComponent.GetMaterial` _projectilemesh 0)))
  (bind _output_get (set `self.MissileMaterialInstance` _returnvalue))
  (`MaterialInstanceDynamic.SetScalarParameterValue` _output_get "RocketPower" 0.0))