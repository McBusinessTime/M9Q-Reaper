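; Enemy spawner actor that scatters enemies on the ground across its Box component's area at BeginPlay.
; The LineTraceLoop macro runs SpawnCount times, picking random XY points within the box extent and tracing far downward against WorldStatic objects.
; Each blocking hit spawns one Enemy slightly above the ground with random yaw, ignoring collisions, so missed traces spawn nothing.
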(event `self.ReceiveBeginPlay`
  ;[0 0 0] Spawn enemies in box extent
  (bind _hitlocation (`self.LineTraceLoop`)
    (:`Output`
      (`|SpawnActorFromClass` "/Game/MQ9Reaper/Character/Blueprint/Enemy.Enemy_C" (`KismetMathLibrary.MakeTransform` (+ _hitlocation (0.0 0.0 96.0)) (`KismetMathLibrary.MakeRotator` 0.0 0.0 (`KismetMathLibrary.RandomFloatInRange` -180.0 180.0))) "AlwaysSpawn" "OverrideRootScale"))))

(fn `UserConstructionScript`)